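; Greenhouse actor that serves as a debug visualizer and test harness for the grid-based plant simulation in its greenhouse component.
; On BeginPlay it caches the grid size and starts a looping timer that draws each cell as a stage-colored debug point, labeled with a switchable plant stat.
; Debug functions forward planting, watering, lighting, harvesting, dead-plant clearing and simulation stepping to the component, using random or selected targets, and print statistics.
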(event `InitGreenhouse`
  (bind _greenhousecomp (`self.GreenhouseComp`)
    (:`then`
      (set `self.GreenhouseGridHeight` (`GreenhouseComponent.GridHeight` _greenhousecomp))
      (set `self.GreenhouseGridWidth` (`GreenhouseComponent.GridWidth` _greenhousecomp)))
    (:`else`)))

(event `InitVisualization`
  (`self.GreenhouseComp`
    (:`then`
      (bind _returnvalue (`KismetSystemLibrary.K2_SetTimer` null "DrawDebugGrid" (`self.VisualizationTickTime`) true))
      (set `self.VisualizationTimer` _returnvalue))
    (:`else`)))

(event `self.ReceiveBeginPlay`
  (`self.InitGreenhouse`)
  (`self.InitVisualization`))

(fn `Debug_GetStatistics`
  (bind _selectedplantrowname (`self.SelectedPlantRowName`))
  (bind _greenhousecomp (`self.GreenhouseComp`)
    (:`then`
      (`KismetSystemLibrary.PrintString` (`KismetStringLibrary.Concat_StrStr` "Statistics:  " "Cells occupied - " (`KismetStringLibrary.Conv_IntToString` (`GreenhouseComponent.GetOccupiedCount` _greenhousecomp)) " Ready to harvest - " (`KismetStringLibrary.Conv_IntToString` (`GreenhouseComponent.GetReadyToHarvestCount` _greenhousecomp)) " Problematic cells - " (`KismetStringLibrary.Conv_IntToString` (`GreenhouseComponent.GetProblematicCellsCount` _greenhousecomp)) " Avg water level - " (`KismetStringLibrary.Conv_DoubleToString` (`GreenhouseComponent.GetAverageWaterLevel` _greenhousecomp)) " Amount of plant " (`KismetStringLibrary.Conv_NameToString` _selectedplantrowname) " - " (`KismetStringLibrary.Conv_IntToString` (`GreenhouseComponent.GetPlantCountByType` _greenhousecomp _selectedplantrowname))) true true (struct :`G` 0.56807 :`B` 1.0 :`A` 1.0) 20.0))
    (:`else`)))

(fn `Debug_HarvestPlantSelected`
  (bind _greenhousecomp (`self.GreenhouseComp`)
    (:`then`
      (`GreenhouseComponent.HarvestAt` _greenhousecomp (`self.TargetX`) (`self.TargetY`)))
    (:`else`)))

(fn `Debug_LightAll`
  (bind _greenhousecomp (`self.GreenhouseComp`)
    (:`then`
      (`GreenhouseComponent.SetLightArea` _greenhousecomp 0 0 (`self.GreenhouseGridWidth`) (`self.GreenhouseGridHeight`) (`KismetMathLibrary.RandomFloatInRange` 5.0 15.0)))
    (:`else`)))

(fn `Debug_LightRandom`
  (bind _greenhousecomp (`self.GreenhouseComp`)
    (:`then`
      (`GreenhouseComponent.SetLightCell` _greenhousecomp (`KismetMathLibrary.RandomIntegerInRange` 0 (- (`self.GreenhouseGridWidth`) 1)) (`KismetMathLibrary.RandomIntegerInRange` 0 (- (`self.GreenhouseGridHeight`) 1)) (`KismetMathLibrary.RandomFloatInRange` 5.0 15.0)))
    (:`else`)))

(fn `Debug_LightSelected`
  (bind _greenhousecomp (`self.GreenhouseComp`)
    (:`then`
      (`GreenhouseComponent.SetLightArea` _greenhousecomp (`self.TargetX`) (`self.TargetY`) (`self.TargetExtendX`) (`self.TargetExtendY`) (`self.TargetLevel`)))
    (:`else`)))

(fn `Debug_PlantRandom`
  (bind _greenhousecomp (`self.GreenhouseComp`)
    (:`then`
      (bind _plantdt (`self.PlantDT`)
        (:`then`
          (bind _outrownames (`DataTableFunctionLibrary.GetDataTableRowNames` _plantdt))
          (`GreenhouseComponent.PlantAt` _greenhousecomp (`KismetMathLibrary.RandomIntegerInRange` 0 (- (`self.GreenhouseGridWidth`) 1)) (`KismetMathLibrary.RandomIntegerInRange` 0 (- (`self.GreenhouseGridHeight`) 1)) (`KismetArrayLibrary.Array_Random` _outrownames)))
        (:`else`)))
    (:`else`)))

(fn `Debug_PlantSelected`
  (bind _greenhousecomp (`self.GreenhouseComp`)
    (:`then`
      (`GreenhouseComponent.PlantAt` _greenhousecomp (`self.TargetX`) (`self.TargetY`) (`self.SelectedPlantRowName`)))
    (:`else`)))

(fn `Debug_ProceedSimulation`
  (bind _returnvalue (`KismetMathLibrary.FCeil` (`self.TargetLevel`)))
  (bind _greenhousecomp (`self.GreenhouseComp`)
    (:`then`
      (if (> _returnvalue 0)
        (`GreenhouseComponent.StepSimulation` _greenhousecomp _returnvalue)))
    (:`else`)))

(fn `Debug_RemoveDeadPlants`
  (bind _greenhousecomp (`self.GreenhouseComp`)
    (:`then`
      (`GreenhouseComponent.ClearDead` _greenhousecomp))
    (:`else`)))

(fn `Debug_ShowGrowth`
  (set `self.VisualizationMode` 3))

(fn `Debug_ShowHealth`
  (set `self.VisualizationMode` 4))

(fn `Debug_ShowLight`
  (set `self.VisualizationMode` 2))

(fn `Debug_ShowName`
  (set `self.VisualizationMode` 0))

(fn `Debug_ShowWater`
  (set `self.VisualizationMode` 1))

(fn `Debug_WaterAll`
  (bind _greenhousecomp (`self.GreenhouseComp`)
    (:`then`
      (`GreenhouseComponent.WaterArea` _greenhousecomp 0 0 (`self.GreenhouseGridWidth`) (`self.GreenhouseGridHeight`) (`KismetMathLibrary.RandomFloatInRange` 5.0 15.0)))
    (:`else`)))

(fn `Debug_WaterRandom`
  (bind _greenhousecomp (`self.GreenhouseComp`)
    (:`then`
      (`GreenhouseComponent.WaterCell` _greenhousecomp (`KismetMathLibrary.RandomIntegerInRange` 0 (- (`self.GreenhouseGridWidth`) 1)) (`KismetMathLibrary.RandomIntegerInRange` 0 (- (`self.GreenhouseGridHeight`) 1)) (`KismetMathLibrary.RandomFloatInRange` 5.0 15.0)))
    (:`else`)))

(fn `Debug_WaterSelected`
  (bind _greenhousecomp (`self.GreenhouseComp`)
    (:`then`
      (`GreenhouseComponent.WaterArea` _greenhousecomp (`self.TargetX`) (`self.TargetY`) (`self.TargetExtendX`) (`self.TargetExtendY`) (`self.TargetLevel`)))
    (:`else`)))

(fn `DrawDebugGrid`
  (locals (Y :type Integer) (X :type Integer) (PlantData :type "PlantData Structure") (SpawnColor :type "LinearColor Structure") (GreenhouseCell :type "GreenhouseCell Structure") (SpawnLocation :type "Vector Structure") (PlantFound :type Boolean :default false))
  (bind (_returnvalue_x _returnvalue_y _returnvalue_z) (`KismetMathLibrary.BreakVector` (`self.K2_GetActorLocation`)))
  (bind _cellsize (`self.CellSize`))
  (bind _cellsize_2 (`self.CellSize`))
  (bind _greenhousecomp (`self.GreenhouseComp`))
  (bind (_spawnlocation_x _spawnlocation_y _spawnlocation_z) (`KismetMathLibrary.BreakVector` (`local.SpawnLocation`)))
  (bind (_plantrowname _waterlevel _lightlevel _growthprogress _stage) (break `GreenhouseCell` (`local.GreenhouseCell`)))
  (bind (_plantrowname_2 _waterlevel_2 _lightlevel_2 _growthprogress_2 _stage_2 _planthealth) (break `GreenhouseCell` (`local.GreenhouseCell`)))
  (bind (_outcell _returnvalue) (`GreenhouseComponent.GetCellData` _greenhousecomp (`local.X`) (`local.Y`)))
  (bind _returnvalue_2 (/ (`self.CellSize`) 2.0))
  (bind (_outdata _bfound) (`GreenhouseComponent.GetPlantStats` _greenhousecomp _plantrowname))
  (for _index (range (`self.GreenhouseGridHeight`))
    (set `local.Y` _index)
    (for _index_2 (range (`self.GreenhouseGridWidth`))
      (set `local.X` _index_2)
      (if _returnvalue
        (set `local.GreenhouseCell` _outcell)
        (set `local.PlantFound` _bfound)
        (if (`local.PlantFound`)
          (set `local.PlantData` _outdata)
          (else
            (set `local.PlantData` (struct))))
        (set `local.SpawnColor` (select `EPlantStages` _stage :`Empty` (struct :`R` 1.0 :`G` 1.0 :`B` 1.0 :`A` 1.0) :`Seed` (struct :`G` 0.888759 :`B` 1.0 :`A` 1.0) :`Growing` (struct :`R` 1.0 :`G` 0.930137 :`A` 1.0) :`ReadyToHarvest` (struct :`R` 0.031093 :`G` 1.0 :`A` 1.0) :!type "LinearColor Structure"))
        (set `local.SpawnLocation` (`KismetMathLibrary.MakeVector` (+ (* (- (`local.Y`) (/ (`self.GreenhouseGridHeight`) 2)) _cellsize 2.0) (* _cellsize 0.5) _returnvalue_y) (+ (* (- (`local.X`) (/ (`self.GreenhouseGridWidth`) 2)) _cellsize_2 2.0) (* _cellsize_2 0.5) _returnvalue_x) (+ _returnvalue_z (`self.VisualizationHeightOffset`))))
        (`KismetSystemLibrary.DrawDebugPoint` (`local.SpawnLocation`) (`self.CellSize`) (`local.SpawnColor`) (`self.VisualizationTickTime`))
        (if (`local.PlantFound`)
          (`KismetSystemLibrary.DrawDebugString` (`KismetMathLibrary.MakeVector` (+ _spawnlocation_x _returnvalue_2) (+ _spawnlocation_y _returnvalue_2) _spawnlocation_z) (select `byte` (`self.VisualizationMode`) :`0` (`KismetTextLibrary.Conv_TextToString` (`.DisplayName` (break `PlantData` (`local.PlantData`)))) :`1` (`KismetStringLibrary.Conv_DoubleToString` _waterlevel_2) :`2` (`KismetStringLibrary.Conv_DoubleToString` _lightlevel_2) :`3` (`KismetStringLibrary.Conv_DoubleToString` _growthprogress_2) :`4` (`KismetStringLibrary.Conv_DoubleToString` _planthealth)) null (`local.SpawnColor`) (`self.VisualizationTickTime`)))))))

(fn `UserConstructionScript`)